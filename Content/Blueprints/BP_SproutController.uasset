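; Player controller that views the level through a placed CameraActor and lets the player drag physics components with the cursor.
; Each tick, while not grabbing, it traces one object type under the cursor to track the hovered component.
; The Grab input attaches a PhysicsHandle to a hovered component tagged "grab" and releases it on button up.
; While held, the handle target follows the cursor hit in XY at a fixed world height.
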(event EventBeginPlay
  (bind _outactors (Actor|GetAllActorsOfClass "/Script/Engine.CameraActor"))
  (for _array_element _outactors
    (Game|Player|SetViewTargetwithBlend _array_element 0.0 "VTBlend_Linear" 0.0 false)))

(event EventTick
  (params (DeltaSeconds :type Float%20%28single-precision%29))
  (Utilities|FlowControl|Sequence
    (:then_0
      (CallFunction|TraceInteraction))
    (:then_1
      (CallFunction|UpdatePhysicsHandle))))

(event Input|ActionEvents|InputActionGrab
  (params (Key :type Key%20Structure :default "None"))
  (:Pressed
    (CallFunction|Grab))
  (:Released
    (CallFunction|Release)))

(fn ConstructionScript)

(fn Grab
  (bind _hoveredcomponent (Variables|Default|GetHoveredComponent))
  (bind _hoveredcomponent_2 (Variables|Default|GetHoveredComponent)
    (:then
      (if (Components|ComponentHasTag _hoveredcomponent_2 "grab")
        (Utilities|FlowControl|Sequence
          (:then_0
            (Class|PhysicsHandleComponent|GrabComponentatLocation (Variables|Default|GetPhysicsHandle) _hoveredcomponent "None" (Transformation|GetWorldLocation _hoveredcomponent))
            (Development|PrintString (Utilities|String|Append "Grab " (Utilities|GetDisplayName _hoveredcomponent))))
          (:then_1
            (Variables|Default|SetisGrabbing true)))))
    (:else)))

(fn TraceInteraction
  (bind _array (Utilities|Array|MakeArray "ObjectTypeQuery7"))
  (bind (_hitresult _returnvalue) (Class|PlayerController|GetHitResultUnderCursorforObjects _array false))
  (bind (_bblockinghit _binitialoverlap _time _distance _location _impactpoint _normal _impactnormal _physmat _hitactor _hitcomponent) (Collision|BreakHitResult _hitresult))
  (if (not (Variables|Default|GetisGrabbing))
    (if _returnvalue
      (if (!= (Variables|Default|GetHoveredComponent) _hitcomponent)
        (Variables|Default|SetHoveredActor _hitactor)
        (Variables|Default|SetHoveredComponent _hitcomponent))
      (else
        (Variables|Default|SetHoveredActor 0)
        (Variables|Default|SetHoveredComponent 0)))))

(fn UpdatePhysicsHandle
  (bind _array (Utilities|Array|MakeArray "ObjectTypeQuery1" "ObjectTypeQuery2" "ObjectTypeQuery3" "ObjectTypeQuery4" "ObjectTypeQuery6"))
  (bind (_hitresult _returnvalue) (Class|PlayerController|GetHitResultUnderCursorforObjects _array false))
  (bind _location (Collision|BreakHitResult _hitresult))
  (bind (_x _y) (Class|KismetMathLibrary|BreakVector3f _location))
  (if (Variables|Default|GetisGrabbing)
    (if _returnvalue
      (Physics|Components|PhysicsHandle|SetTargetLocation (Variables|Default|GetPhysicsHandle) (Math|Vector|MakeVector _x _y (+ 0.0 2e+02))))))

(fn Release
  (if (Variables|Default|GetisGrabbing)
    (Physics|Components|PhysicsHandle|ReleaseComponent (Variables|Default|GetPhysicsHandle))
    (Variables|Default|SetisGrabbing false)
    (Variables|Default|SetGrabbedActor 0)))